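; Blueprint that hosts a MANN neural network component and prepares its trained parameters for runtime use.
; The construction script points the network's folder at DeepLearning/trained/ inside the project content directory.
; On BeginPlay it calls StoreParameters, then LoadParameters on that component.
; A LoadParametersFiles branch and a second store call are left unwired.
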(event `self.ReceiveBeginPlay`
  (bind _mann (`self.MANN`))
  (`NeuralNetworkComponent.StoreParameters` _mann)
  (`NeuralNetworkComponent.LoadParameters` _mann))

(fn `UserConstructionScript`
  (set `NeuralNetworkComponent.Folder` (`KismetStringLibrary.Concat_StrStr` (`KismetSystemLibrary.GetProjectContentDirectory`) "DeepLearning/trained/") (`self.MANN`)))